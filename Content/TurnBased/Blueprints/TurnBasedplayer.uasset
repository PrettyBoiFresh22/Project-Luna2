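; Player pawn for turn-based battles that lets the player pick combat characters with the mouse.
; While possessed it shows the cursor and a character control widget, and removes the widget when unpossessed.
; Each tick a Visibility trace from the cursor records the hovered actor if it matches the combat character class, and left click makes it the selected actor.
; SwitchTurn toggles the current turn between player and enemy.
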(event EventBeginPlay
  ;[1 1 1] Changes all necessary settings here
  (bind _returnvalue (UserInterface|CreateWidget "/Game/TurnBased/Blueprints/CharacterWidget.CharacterWidget_C"))
  (bind _output_get (Variables|Default|SetControlMenu _returnvalue))
  (if (Class|Pawn|IsControlled)
    (Variables|/Script/Engine.PlayerController|SetbShowMouseCursor (.AsPossessor%20Control (Utilities|Casting|CastToPossessorControl (Game|GetPlayerController 0))) true)
    (UserInterface|Viewport|AddtoViewport _output_get 0)
    (Development|PrintString "Current Turn")
    (Development|PrintString (Utilities|String|EnumtoString (Variables|Default|GetCurrentTurn)))))

(event EventPossessed
  (params (NewController :type Controller%20Object%20Reference))
  ;[1 1 1] Changes all necessary settings here
  (Variables|/Script/Engine.PlayerController|SetbShowMouseCursor (.AsPossessor%20Control (Utilities|Casting|CastToPossessorControl (Game|GetPlayerController 0))) true)
  (UserInterface|Viewport|AddtoViewport (stale EventBeginPlay _output_get) 0)
  (Development|PrintString "Current Turn")
  (Development|PrintString (Utilities|String|EnumtoString (Variables|Default|GetCurrentTurn))))

(event EventUnpossessed
  (params (OldController :type Controller%20Object%20Reference))
  ;[1 1 1] Changes all necessary settings here
  (Widget|RemovefromParent (stale EventBeginPlay _returnvalue)))

(event EventTick
  (params (DeltaSeconds :type Float%20%28single-precision%29))
  (bind _returnvalue (Game|GetPlayerController 0))
  (bind (_worldlocation _worlddirection) (Game|Player|ConvertMouseLocationToWorldSpace _returnvalue))
  ;[1 1 1] The mouse is raycast to in order to select pawns on the area that is given during a battle
  (bind _outhit (Collision|LineTraceByChannel _worldlocation (+ _worldlocation (* _worlddirection (Variables|Default|GetRaycastMouseDist))) "TraceTypeQuery1" false 0 "None"))
  ;[1 1 1] Checks to see if the object the mouse raycasts to is the exact same class as the CombatChar class
  (if (Utilities|ClassIsChildOf (Utilities|GetClass (.hitactor _outhit)) (Variables|Default|GetClassReference))
    (Variables|Default|SetHoveredActor (.hitactor _outhit))))

(event Input|MouseEvents|LeftMouseButton
  (params (Key :type Key%20Structure :default "None"))
  ;[1 1 1] Sets the actor to be the current selected actor and will later be parsed as a class of CombatChar
  (:Pressed
    (if (Utilities|ClassIsChildOf (Utilities|GetClass (.hitactor (stale EventTick _outhit))) (Variables|Default|GetClassReference))
      (bind _output_get (Variables|Default|SetSelectedActor (Variables|Default|GetHoveredActor)))
      (Development|PrintString (Utilities|GetDisplayName _output_get)))))

(fn ConstructionScript)

(fn SwitchTurn
  (switch Utilities|FlowControl|Switch|SwitchonTurnEnums (Variables|Default|GetCurrentTurn)
    (:NewEnumerator0
      (Variables|Default|SetCurrentTurn "NewEnumerator1"))
    (:NewEnumerator1
      (Variables|Default|SetCurrentTurn "NewEnumerator0"))))