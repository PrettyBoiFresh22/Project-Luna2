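; Debug possession switcher that toggles the player between third-person and turn-based control.
; Tab possesses the first BP_ThirdPersonCharacter found in the world, switches to game-only input and hides the mouse cursor.
; The 1 key possesses the first TurnBasedplayer found and switches to game-and-UI input focused on a widget, without re-showing the cursor.
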(event EventBeginPlay)

(event EventTick
  (params (DeltaSeconds :type Float%20%28single-precision%29)))

(event Input|KeyboardEvents|DebugKeyTab
  (params (Key :type Key%20Structure :default "None") (ActionValue :type Input%20Action%20Value%20Structure))
  (bind _returnvalue (Game|GetPlayerController 0))
  (:Pressed
    (bind _outactors (Actor|GetAllActorsOfClass "/Game/ThirdPerson/Blueprints/BP_ThirdPersonCharacter.BP_ThirdPersonCharacter_C"))
    (Pawn|Possess _returnvalue (Utilities|Array|Get(acopy) _outactors))
    (Input|SetInputModeGameOnly _returnvalue true)
    (Variables|Default|SetbShowMouseCursor false)))

(event Input|KeyboardEvents|1
  (params (Key :type Key%20Structure :default "None"))
  (bind _returnvalue (Game|GetPlayerController 0))
  (:Pressed
    (bind _outactors (Actor|GetAllActorsOfClass "/Game/TurnBased/Blueprints/TurnBasedplayer.TurnBasedplayer_C"))
    (Pawn|Possess _returnvalue (Utilities|Array|Get(acopy) _outactors))
    (Input|SetInputModeGameandUI _returnvalue (Variables|Default|GetWidget) "DoNotLock" true false)))

(fn ConstructionScript)