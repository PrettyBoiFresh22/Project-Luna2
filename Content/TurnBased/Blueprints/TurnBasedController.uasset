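; TurnBasedController handles mouse selection of combat characters during turn-based battles.
; On BeginPlay it shows the cursor, sets an attack stat and caches the player pawn as BP_CombatCharBasic for class comparison.
; Each tick it traces from the mouse, storing hits of exactly that pawn's class as HoveredActor, which is never cleared on a miss.
; Left-click copies HoveredActor into SelectedActor and prints its name.
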(event EventBeginPlay
  ;[1 1 1] Changes all necessary settings here
  (Variables|Default|SetbShowMouseCursor true)
  (Variables|Default|SetAttack_Stat 10)
  ;[1 1 1] Will pull the OpponentPawn class in order to act as a comparision to confirm a given component is the OpponentPawn class
  (bind _asbp_combat_char_basic (Utilities|Casting|CastToBP_CombatCharBasic (Game|Player|GetPlayerPawn 0))))

(event EventTick
  (params (DeltaSeconds :type Float%20%28single-precision%29))
  (bind _returnvalue (Game|GetPlayerController 0))
  (bind (_worldlocation _worlddirection) (Game|Player|ConvertMouseLocationToWorldSpace _returnvalue))
  ;[1 1 1] The mouse is raycast to in order to select pawns on the area that is given during a battle
  (bind _output_get (Variables|Default|SetMouse%20Line 100000))
  (bind _outhit (Collision|LineTraceByChannel _worldlocation (+ _worldlocation (* _worlddirection _output_get)) "TraceTypeQuery1" false 0 "None"))
  ;[1 1 1] Checks to see if the object the mouse raycasts to is the exact same class as the OpponentPawn class
  (if (== (Utilities|GetClass (stale EventBeginPlay _asbp_combat_char_basic)) (Utilities|GetClass (.hitactor _outhit)))
    (Variables|Default|SetHovered_Actor (.hitactor _outhit))))

(event Input|MouseEvents|LeftMouseButton
  (params (Key :type Key%20Structure))
  ;[1 1 1] After the object is confirmed to be a character, it will set this as a selected actor and is able to be communicated by other blueprints
  (:Pressed
    (bind _output_get (Variables|Default|SetSelected_Actor (Variables|Default|GetHovered_Actor)))
    (Development|PrintString (Utilities|GetDisplayName _output_get))))

(fn ConstructionScript)